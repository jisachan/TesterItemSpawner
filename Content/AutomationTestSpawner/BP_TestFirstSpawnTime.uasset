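; Functional test that checks whether an item spawner's first spawn respects its configured FirstSpawnDelay.
; PrepareTest records the current time and binds to the ItemSpawnManager's OnSpawn delegate, then StartTest starts spawning.
; On spawn, it compares the time elapsed since preparation to the delay within a small tolerance and finishes the test as succeeded or failed.
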(event Custom|OnSpawn_Event_0
  (Variables|Default|SetTimeInSecondsAtFirstSpawn (Utilities|Time|GetTimeSeconds))
  (if (Math|Float|NearlyEqual(Float) (Variables|/Script/ItemSpawnTester.ItemSpawnManager|GetFirstSpawnDelay (Variables|/Game/BP_ItemSpawner.BP_ItemSpawner_C|GetItemSpawnManager (Variables|Default|GetItemSpawner))) (- (Variables|Default|GetTimeInSecondsAtFirstSpawn) (Variables|Default|GetTimeInSecondsBeforeFirstSpawn)) 0.01)
    (Class|FunctionalTest|FinishTest "Succeeded")
    (else
      (Class|FunctionalTest|FinishTest "Failed"))))

(event EventPrepareTest
  (Variables|Default|SetTimeInSecondsBeforeFirstSpawn (Utilities|Time|GetTimeSeconds))
  (EventDispatchers|AssignOnSpawn (Variables|/Game/BP_ItemSpawner.BP_ItemSpawner_C|GetItemSpawnManager (Variables|Default|GetItemSpawner)) (delegate Custom|OnSpawn_Event_0)))

(event EventStartTest
  (Class|ItemSpawnManager|OnStartSpawning (Variables|/Game/BP_ItemSpawner.BP_ItemSpawner_C|GetItemSpawnManager (Variables|Default|GetItemSpawner))))

(fn ConstructionScript)