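; Functional test that checks whether an item spawner reaches its expected total number of spawned items.
; Preparation shortens the spawn cooldown on the spawner's ItemSpawnManager, then test start computes the expected total from the per-type limit times the item type count and begins spawning.
; Tick polls the spawned count and finishes as succeeded on an exact match, with no explicit failure branch.
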(event EventPrepareTest
  (Variables|/Script/ItemSpawnTester.ItemSpawnManager|SetSpawnCooldown (Variables|/Game/BP_ItemSpawner.BP_ItemSpawner_C|GetItemSpawnManager (Variables|Default|GetItemSpawner)) 0.1))

(event EventStartTest
  (bind _itemspawner (Variables|Default|GetItemSpawner))
  (bind _itemspawnmanager (Variables|/Game/BP_ItemSpawner.BP_ItemSpawner_C|GetItemSpawnManager _itemspawner))
  (bind _output_get (Variables|Default|SetTotalNumOfItemsToSpawn (* (Variables|/Script/ItemSpawnTester.ItemSpawnManager|GetSpawnLimitPerType _itemspawnmanager) (Utilities|Array|Length (Variables|/Script/ItemSpawnTester.ItemSpawnManager|GetItemsToSpawn _itemspawnmanager)))))
  (Class|ItemSpawnManager|OnStartSpawning _itemspawnmanager))

(event EventTick
  (params (DeltaSeconds :type Float%20%28single-precision%29))
  (if (== (stale EventStartTest _output_get) (Variables|/Script/ItemSpawnTester.ItemSpawnManager|GetNumOfSpawnedItems (Variables|/Game/BP_ItemSpawner.BP_ItemSpawner_C|GetItemSpawnManager (Variables|Default|GetItemSpawner))))
    (Development|PrintString "Hello")
    (Class|FunctionalTest|FinishTest "Succeeded")))

(fn ConstructionScript)