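; Functional test that checks the recurring spawn timer of an item spawner's ItemSpawnManager.
; Setup sets a fixed cooldown with no first-spawn delay, then derives the expected total time from spawn limit per type, item type count, cooldown and items per spawn.
; It timestamps the first spawn and the finish event, passing if the elapsed time matches the expected total within a small tolerance.
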(event Custom|OnAllSpawnsFinished
  (bind _output_get (Variables|Default|SetTimeInSecondsWhenAllSpawnsFinish (Utilities|Time|GetTimeSeconds)))
  (if (Math|Float|NearlyEqual(Float) (- _output_get (Variables|Default|GetTimeInSecondsOnFirstSpawn)) (Variables|Default|GetTotalSpawnTime) 0.1)
    (Class|FunctionalTest|FinishTest "Succeeded")
    (else
      (Class|FunctionalTest|FinishTest "Failed"))))

(event Custom|OnFirstSpawn
  (Utilities|FlowControl|DoOnce false
    (:Completed
      (Variables|Default|SetTimeInSecondsOnFirstSpawn (Utilities|Time|GetTimeSeconds)))))

(event EventPrepareTest
  (bind _itemspawner (Variables|Default|GetItemSpawner))
  (bind _itemspawnmanager (Variables|/Game/BP_ItemSpawner.BP_ItemSpawner_C|GetItemSpawnManager _itemspawner))
  (EventDispatchers|BindEventtoOnSpawnFinish _itemspawnmanager (delegate Custom|OnAllSpawnsFinished))
  (EventDispatchers|BindEventtoOnSpawn _itemspawnmanager (delegate Custom|OnFirstSpawn))
  (bind _output_get (Variables|/Script/ItemSpawnTester.ItemSpawnManager|SetSpawnCooldown _itemspawnmanager 0.5))
  (Variables|/Script/ItemSpawnTester.ItemSpawnManager|SetFirstSpawnDelay _itemspawnmanager 0.0)
  (bind _output_get_2 (Variables|Default|SetTotalNumOfItemsToSpawn (* (Variables|/Script/ItemSpawnTester.ItemSpawnManager|GetSpawnLimitPerType _itemspawnmanager) (Utilities|Array|Length (Variables|/Script/ItemSpawnTester.ItemSpawnManager|GetItemsToSpawn _itemspawnmanager)))))
  (Variables|Default|SetTotalSpawnTime (/ (* _output_get_2 _output_get) (Math|Conversions|ToFloat(Integer) (Variables|/Script/ItemSpawnTester.ItemSpawnManager|GetNumOfItemsPerSpawn _itemspawnmanager)))))

(event EventStartTest
  (Class|ItemSpawnManager|OnStartSpawning (Variables|/Game/BP_ItemSpawner.BP_ItemSpawner_C|GetItemSpawnManager (Variables|Default|GetItemSpawner))))

(fn ConstructionScript)