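; Functional test that verifies an item spawner produces its configured number of items per spawn.
; On prepare, it binds to the spawn manager's per-item and spawn-finished events and resets a counter.
; The test starts spawning, increments and prints the count for each spawned item, then succeeds only if the final count equals NumOfItemsPerSpawn.
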(event Custom|OnCurrentSpawnFinished
  (if (== (Variables|/Script/ItemSpawnTester.ItemSpawnManager|GetNumOfItemsPerSpawn (Variables|/Game/BP_ItemSpawner.BP_ItemSpawner_C|GetItemSpawnManager (Variables|Default|GetItem%20Spawner))) (Variables|Default|GetSpawnedItemsNum))
    (Class|FunctionalTest|FinishTest "Succeeded")
    (else
      (Class|FunctionalTest|FinishTest "Failed"))))

(event Custom|OnCurrentSpawnedItem_Event_0
  (bind _result (Math|Integer|IncrementInt (Variables|Default|GetSpawnedItemsNum))
    (:%20%20
      (Development|PrintString (Utilities|String|ToString(Integer) _result)))))

(event EventPrepareTest
  (bind _item_spawner (Variables|Default|GetItem%20Spawner))
  (bind _itemspawnmanager (Variables|/Game/BP_ItemSpawner.BP_ItemSpawner_C|GetItemSpawnManager _item_spawner))
  (EventDispatchers|AssignOnCurrentSpawnedItem _itemspawnmanager (delegate Custom|OnCurrentSpawnedItem_Event_0))
  (EventDispatchers|BindEventtoOnCurrentSpawnFinished _itemspawnmanager (delegate Custom|OnCurrentSpawnFinished))
  (Variables|Default|SetSpawnedItemsNum 0))

(event EventStartTest
  (Class|ItemSpawnManager|OnStartSpawning (Variables|/Game/BP_ItemSpawner.BP_ItemSpawner_C|GetItemSpawnManager (Variables|Default|GetItem%20Spawner))))

(fn ConstructionScript)